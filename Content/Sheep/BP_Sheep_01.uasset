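; Sheep AI actor with random size that wanders, grazes on BP_Grass, follows the player when music is heard, and can be put to sleep.
; A Tick-driven state switch runs each behavior via AIMoveTo and poses the head per state.
; Sight perception finds the nearest untargeted grass, claims it, and a head sphere trace triggers eating.
; "Music" stimuli release the grass and override all states except sleep until a timer ends.
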(event `self.ReceiveBeginPlay`
  (bind _returnvalue (`KismetMathLibrary.RandomFloatInRange` 0.8 1.2))
  (`|ExecutionSequence`
    (:`then_0`
      ;[1 1 1] Randomize mesh size between 80-120%
      (`SceneComponent.SetWorldScale3D` (`self.Mesh`) (`KismetMathLibrary.MakeVector` _returnvalue _returnvalue _returnvalue)))
    (:`then_1`
      (bind _outactors (`GameplayStatics.GetAllActorsOfClass` "/Script/Landscape.Landscape"))
      (set `self.LandscapeArray` _outactors))))

(event `self.ReceiveTick`
  (params (DeltaSeconds :type "Float (single-precision)"))
  (bind _head (`self.Head`))
  (bind _head_2 (`self.Head`))
  (bind _head_3 (`self.Head`))
  (bind _head_4 (`self.Head`))
  (`/Engine/EditorBlueprintResources/StandardMacros.IsValid` self
    (:`Is Valid`
      (`|ExecutionSequence`
        (:`then_0`
          ;[1 1 1] STATE SWITCH
          (switch `string` (`self.STATE`)
            (:`IDLE`
              (`self.IDLE`)
              (`/Engine/EditorBlueprintResources/StandardMacros.IsValid` _head_3 :!label _label
                (:`Is Valid`
                  (`SceneComponent.K2_SetRelativeRotation` _head_3 (struct :`Pitch` 180.0) false false))))
            (:`WANDER`
              (`self.Wander`)
              (goto _label))
            (:`FOLLOWMUSIC`
              (`self.FollowMusic`)
              (goto _label))
            (:`MOVETOGRASSTARGET`
              (`self.MOVETOGRASSTARGET`)
              (`/Engine/EditorBlueprintResources/StandardMacros.IsValid` _head_2
                (:`Is Valid`
                  (`SceneComponent.K2_SetRelativeRotation` _head_2 (struct :`Pitch` 210.0) false false))))
            (:`EATGRASS`
              (`self.EATGRASS`)
              (`/Engine/EditorBlueprintResources/StandardMacros.IsValid` _head_4
                (:`Is Valid`
                  (`SceneComponent.K2_SetRelativeRotation` _head_4 (struct :`Pitch` 140.0) false false))))
            (:`SLEEP`
              (`self.SLEEP`)
              (`/Engine/EditorBlueprintResources/StandardMacros.IsValid` _head
                (:`Is Valid`
                  (`SceneComponent.K2_SetRelativeRotation` _head (struct :`Pitch` 120.0) false false))))))
        (:`then_1`
          (if (`self.IsDead`)
            (`self.K2_DestroyActor`)))))))

(event `self.AIPerception.OnTargetPerceptionUpdated`
  (params (Actor :type "Actor Object Reference") (Stimulus :type "AIStimulus Structure"))
  ;[1 1 1] Hear/"Un"Hear Music
  (if (`KismetStringLibrary.NotEqual_StrStr` (`self.STATE`) "SLEEP")
    (if (== Stimulus_Tag "Music")
      (`KismetSystemLibrary.K2_SetTimerDelegate` (delegate `CantHearMusic`) 1.5)
      (set `self.HearsMusic` true)
      (`self.UnassignGrassTarget`
        (:`then`
          _)
        (:`Is Not Valid`
          _))
      (set `self.STATE` "FOLLOWMUSIC"))))

(event `CantHearMusic`
  ;[1 1 1] Hear/"Un"Hear Music
  (set `self.HearsMusic` false)
  (set `self.STATE` "IDLE")
  (`self.GetAvailableGrass`))

(event `IDLE`
  ;[1 1 1] IDLE State
  (if (< (`self.CurrentWaitTime`) (`self.IdleWaitTime`))
    (set `self.CurrentWaitTime` (+ (`self.CurrentWaitTime`) 1.0))
    (else
      (`self.GetWanderVector`)
      (set `self.STATE` "WANDER")
      (`self.GetAvailableGrass`))))

(event `GetWanderVector`
  ;[1 1 1] Get Wander Vector
  (bind _randomlocation (`NavigationSystemV1.K2_GetRandomLocationInNavigableRadius` (`self.K2_GetActorLocation`) 500.0 null null))
  (set `self.WanderVector` _randomlocation))

(event `GetAvailableGrass`
  ;[1 1 1] GETAVAILABLE GRASS ARRAY
  (`KismetArrayLibrary.Array_Clear` (`self.GrassArray`))
  (for _array_element (`AIPerceptionComponent.GetCurrentlyPerceivedActors` (`self.AIPerception`) "/Script/AIModule.AISense_Sight") :!label _label_2
    (bind _asbp_grass (cast `/Game/GrassSpawner/BP_Grass` _array_element))
    (if (not (`/Game/GrassSpawner/BP_Grass.IsTargeted` _asbp_grass))
      (`KismetArrayLibrary.Array_Add` (`self.GrassArray`) _asbp_grass)
      (if (>= (`KismetArrayLibrary.Array_Length` (`self.GrassArray`)) (`self.GrassArraySizeLimit`))
        (`self.BreakGrassArrayLoop`))))
  (`self.GetCLosestGrassTarget`))

(event `WANDER`
  ;[1 1 1] WANDER State
  (`|AIMoveTo` self (`self.WanderVector`) null 100.0
    (:`OnSuccess`
      (set `self.IdleWaitTime` (`KismetMathLibrary.RandomFloatInRange` 30.0 120.0))
      (set `self.CurrentWaitTime` 0.0)
      (set `self.STATE` "IDLE"))))

(event `BreakGrassArrayLoop`
  ;[1 1 1] GETAVAILABLE GRASS ARRAY
  (goto _label_2 :!via `Break`))

(event `FOLLOWMUSIC`
  ;[1 1 1] FOLLOWMUSIC State
  (`|AIMoveTo` self (`self.K2_GetActorLocation` (`GameplayStatics.GetPlayerPawn` 0)) null 50.0))

(event `GetClosestGrassTarget`
  ;[1 1 1] SET GRASS TARGET
  (bind _asbp_grass (cast `/Game/GrassSpawner/BP_Grass` (`.ReturnValue` (`GameplayStatics.FindNearestActor` (`self.K2_GetActorLocation`) (`self.GrassArray`))))
    (:`then`
      (bind _output_get (set `self.GrassTarget` _asbp_grass))
      (set `/Game/GrassSpawner/BP_Grass.IsTargeted` true _output_get)
      (set `self.GrassVector` (`self.K2_GetActorLocation` (`self.GrassTarget`)))
      (set `self.STATE` "MOVETOGRASSTARGET"))
    (:`CastFailed`
      (`self.GetWanderVector`)
      (set `self.STATE` "WANDER"))))

(event `SleepSheep`
  ;[1 1 1] Put Sheep To Sleep
  (`MovementComponent.StopMovementImmediately` (`self.CharacterMovement`))
  (`SceneComponent.K2_SetRelativeLocation` (`self.Body`) (0.0 0.0 -30.0) false false)
  (set `self.STATE` "SLEEP"))

(event `MOVETOGRASSTARGET`
  (bind (_returnvalue_x _returnvalue_y _returnvalue_z) (`KismetMathLibrary.BreakVector` (`SceneComponent.K2_GetComponentLocation` (`self.Head`))))
  ;[1 1 1] MOVETOGRASSTARGET state
  (`|AIMoveTo` self (0.0 0.0 0.0) (`self.GrassTarget`)
    (:`then`
      (bind _outhit (`KismetSystemLibrary.SphereTraceSingle` (`KismetMathLibrary.MakeVector` _returnvalue_x _returnvalue_y _returnvalue_z) (`KismetMathLibrary.MakeVector` (- _returnvalue_x 20.0) _returnvalue_y _returnvalue_z) 20.0 "TraceTypeQuery1" true (`self.LandscapeArray`)))
      (if (== (`.HitActor` (`GameplayStatics.BreakHitResult` _outhit)) (`self.GrassTarget`))
        (`MovementComponent.StopMovementImmediately` (`self.CharacterMovement`))
        (set `self.STATE` "EATGRASS")))))

(event `WakeSheep`
  ;[1 1 1] Wake Sheep Up, set IDLE
  (`SceneComponent.K2_SetRelativeLocation` (`self.Body`) (0.0 0.0 0.0) false false)
  (set `self.STATE` "IDLE"))

(event `EATGRASS`
  ;[1 1 1] EATGRASS state
  (`/Engine/EditorBlueprintResources/StandardMacros.IsValid` (`self.GrassTarget`)
    (:`Is Valid`
      (set `self.Hunger` (+ (`self.Hunger`) (`self.HungerFOODRESTORE`)))
      (if (< (`self.GetDistanceTo` (`self.GrassTarget`) self) 200.0)
        (set `/Game/GrassSpawner/BP_Grass.BeingEaten` true (`self.GrassTarget`))
        (`SceneComponent.K2_SetRelativeRotation` (`self.Head`) (struct :`Pitch` 110.0) false false)
        (else
          (set `/Game/GrassSpawner/BP_Grass.BeingEaten` false (`self.GrassTarget`))
          (`self.GetAvailableGrass`))))
    (:`Is Not Valid`
      (`self.GetAvailableGrass`))))

(event `SLEEP`)

(fn `SetState`
  (if (`self.SeesWolf`)
    (set `self.STATE` "RUNFROMWOLF")
    (elif (`self.HearsMusic`)
      (set `self.STATE` "FOLLOWMUSIC")
      (else
        (set `self.STATE` "IDLE")))))

(fn `UserConstructionScript`)