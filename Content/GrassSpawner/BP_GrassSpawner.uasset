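; BP_GrassSpawner is an actor that populates the area around itself with BP_Grass during the day.
; While DayTime is true, each Tick attempts one spawn, provided both the OwnedGrass count and CurrentGrass are below MaxGrass.
; A downward visibility trace between independently randomized XY offsets finds a spot, accepting only the PM_Grass physical material.
; New grass spawns slightly sunken with random yaw, references its parent spawner and joins OwnedGrass.
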(event `self.ReceiveTick`
  (params (DeltaSeconds :type "Float (single-precision)"))
  (if (`self.DayTime`)
    (`self.SpawnGrassInRadius`)))

(fn `SpawnGrassInRadius`
  (bind (_returnvalue_roll _returnvalue_pitch _returnvalue_yaw) (`KismetMathLibrary.BreakRotator` (`KismetMathLibrary.RandomRotator` false)))
  (bind (_returnvalue_x _returnvalue_y _returnvalue_z) (`KismetMathLibrary.BreakVector` (`self.K2_GetActorLocation`)))
  (bind _returnvalue (+ _returnvalue_y (`KismetMathLibrary.RandomFloatInRange` (`self.MinPosition`) (`self.MaxPosition`))))
  (bind _returnvalue_2 (+ _returnvalue_x (`KismetMathLibrary.RandomFloatInRange` (`self.MinPosition`) (`self.MaxPosition`))))
  (if (< (`KismetArrayLibrary.Array_Length` (`self.OwnedGrass`)) (`self.Max_Grass`))
    (if (< (`self.Current_Grass`) (`self.Max_Grass`))
      (bind _outhit (`KismetSystemLibrary.LineTraceSingle` (`KismetMathLibrary.MakeVector` _returnvalue_2 _returnvalue (+ _returnvalue_z (`self.StartZOffset`))) (`KismetMathLibrary.MakeVector` _returnvalue_2 _returnvalue (- _returnvalue_z (`self.EndZOffset`))) "TraceTypeQuery1"))
      (bind (_bblockinghit _binitialoverlap _time _distance _location _impactpoint _normal _impactnormal _physmat) (`GameplayStatics.BreakHitResult` _outhit))
      (if (== _physmat "/Game/GrassSpawner/PM_Grass.PM_Grass")
        (bind _returnvalue_3 (`|SpawnActorFromClass` "/Game/GrassSpawner/BP_Grass.BP_Grass_C" (`KismetMathLibrary.MakeTransform` (`KismetMathLibrary.MakeVector` (.x _location) (.y _location) (+ (.z _location) -5.0)) (`KismetMathLibrary.MakeRotator` 0.0 0.0 _returnvalue_yaw) (1.0 1.0 1.0)) "Undefined" "OverrideRootScale" null null))
        (set `/Game/GrassSpawner/BP_Grass.ParentSpawner` self _returnvalue_3)
        (`KismetArrayLibrary.Array_Add` (`self.OwnedGrass`) _returnvalue_3)))))

(fn `UserConstructionScript`)