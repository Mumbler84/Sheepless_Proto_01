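; Player character with world-axis WASD movement, a visible cursor, a toggleable lantern and music playing.
; Holding right mouse slows walking and switches facing from movement direction to the cursor, using a WorldStatic trace and interpolated yaw on Tick.
; Toggling music also slows walking and starts a looping timer that reports "Music"-tagged noise events at the player's location.
; Interact toggles any BP_BarnGate overlapping the DoorSensor, while Tick sets lantern light intensity.
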(event `self.ReceiveBeginPlay`
  ;[1 1 1] Begin Play Sequence - Set Show Mouse True, Set Orient to Movement True
  (`|ExecutionSequence`
    (:`then_0`
      (set `PlayerController.bShowMouseCursor` true (`GameplayStatics.GetPlayerController` 0)))
    (:`then_1`
      (set `CharacterMovementComponent.bOrientRotationToMovement` true (`self.CharacterMovement`)))))

(event `InputAxis|Up`
  (params (AxisValue :type "Float (single-precision)"))
  ;[1 1 1] WASD Movement
  (`self.AddMovementInput` (`KismetMathLibrary.MakeVector` (* AxisValue (`self.Speed`)))))

(event `InputAxis|RIght`
  (params (AxisValue :type "Float (single-precision)"))
  ;[1 1 1] WASD Movement
  (`self.AddMovementInput` (`KismetMathLibrary.MakeVector` 0.0 (* AxisValue (`self.Speed`)))))

(event `InputAxis|Down`
  (params (AxisValue :type "Float (single-precision)"))
  ;[1 1 1] WASD Movement
  (`self.AddMovementInput` (`KismetMathLibrary.MakeVector` (* AxisValue (`self.Speed`)))))

(event `InputAxis|Left`
  (params (AxisValue :type "Float (single-precision)"))
  ;[1 1 1] WASD Movement
  (`self.AddMovementInput` (`KismetMathLibrary.MakeVector` 0.0 (* AxisValue (`self.Speed`)))))

(event `Key|RightMouseButton`
  (params (Key :type "Key Structure"))
  (bind _charactermovement (`self.CharacterMovement`))
  (bind _charactermovement_2 (`self.CharacterMovement`))
  ;[1 1 1] RMB Toggle Face Mouse/Move Direction
  (:`Pressed`
    (set `CharacterMovementComponent.bOrientRotationToMovement` false _charactermovement)
    (set `CharacterMovementComponent.MaxWalkSpeed` 300.0 _charactermovement_2))
  (:`Released`
    (set `CharacterMovementComponent.bOrientRotationToMovement` true _charactermovement)
    (set `CharacterMovementComponent.MaxWalkSpeed` 800.0 _charactermovement_2)))

(event `self.ReceiveTick`
  (params (DeltaSeconds :type "Float (single-precision)"))
  (bind (_returnvalue_roll _returnvalue_pitch _returnvalue_yaw) (`KismetMathLibrary.BreakRotator` (`self.K2_GetActorRotation`)))
  (bind _pointlight (`self.PointLight`))
  (bind (_worldlocation _worlddirection) (`PlayerController.DeprojectMousePositionToWorld` (`GameplayStatics.GetPlayerController` 0)))
  (`|ExecutionSequence`
    (:`then_0`
      ;[1 1 1] Face Mouse Position
      (if (not (`CharacterMovementComponent.bOrientRotationToMovement` (`self.CharacterMovement`)))
        (bind _outhit (`KismetSystemLibrary.LineTraceSingleForObjects` _worldlocation (+ _worldlocation (* _worlddirection 10000.0)) (`|MakeArray` "ObjectTypeQuery1" :!type "EObjectTypeQuery Enum")))
        (`self.K2_SetActorRotation` (`KismetMathLibrary.RInterpTo` (`KismetMathLibrary.MakeRotator` 0.0 0.0 _returnvalue_yaw) (`KismetMathLibrary.MakeRotator` 0.0 0.0 (.yaw (`KismetMathLibrary.FindLookAtRotation` (`self.K2_GetActorLocation`) (`.ImpactPoint` (`GameplayStatics.BreakHitResult` _outhit))))) DeltaSeconds (`self.LookAtMouseSpeed`)))))
    (:`then_1`
      (if (`self.LanternOn`)
        (`LightComponent.SetIntensity` _pointlight 1000.0)
        (else
          (`LightComponent.SetIntensity` _pointlight 0.0))))))

(event `InputAction|ToggleLantern`
  (params (Key :type "Key Structure"))
  (:`Released`
    (`/Engine/EditorBlueprintResources/StandardMacros.FlipFlop`
      (:`A`
        (set `self.LanternOn` true))
      (:`B`
        (set `self.LanternOn` false)))))

(event `InputAction|Start/Stop Music`
  (params (Key :type "Key Structure"))
  (bind _charactermovement (`self.CharacterMovement`))
  ;[1 1 1] Toggle Music Playing
  (:`Pressed`
    (`/Engine/EditorBlueprintResources/StandardMacros.FlipFlop`
      (:`A`
        (set `self.PlayingMusic?` true)
        (`self.ReportMusicEvent`)
        (bind _returnvalue (`KismetSystemLibrary.K2_SetTimer` null "ReportMusicEvent" 1.0 true))
        (set `CharacterMovementComponent.MaxWalkSpeed` 300.0 _charactermovement))
      (:`B`
        (set `self.PlayingMusic?` false)
        (`KismetSystemLibrary.K2_PauseTimerHandle` _returnvalue)
        (set `CharacterMovementComponent.MaxWalkSpeed` 800.0 _charactermovement)))))

(event `InputAction|Interact`
  (params (Key :type "Key Structure"))
  (:`Released`
    (for _array_element (`PrimitiveComponent.GetOverlappingActors` (`self.DoorSensor`) null)
      (bind _asbp_barn_gate (cast `/Game/Map/BP_BarnGate` _array_element))
      (`/Game/Map/BP_BarnGate.ToggleDoor` _asbp_barn_gate))))

(fn `ReportMusicEvent`
  (`AISense_Hearing.ReportNoiseEvent` (`self.K2_GetActorLocation`) 1.0 self 0.0 "Music"))

(fn `UserConstructionScript`)